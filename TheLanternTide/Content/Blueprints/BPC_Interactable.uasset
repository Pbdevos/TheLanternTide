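; Interactable component that handles player interaction with NPCs and doors and controls the interact marker.
; It caches the BP_Nyra player character on BeginPlay and gates Interact on her IsInsideInteractRange flag.
; Interact switches on type: NPCs start a conversation on Nyra, while doorways open their WorldToLoad level.
; SetMarkerVisibility toggles the marker, sets its raised offset and turns it toward Nyra's camera on each call.
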(event `self.ReceiveBeginPlay`
  (`self.GetNyraRef`))

(fn `GetNyraRef`
  (bind _asbp_nyra (cast `/Game/ThirdPerson/Blueprints/BP_Nyra` (`GameplayStatics.GetPlayerCharacter` 0)))
  (set `self.As BP Nyra` _asbp_nyra))

(fn `Interact`
  (params (InteractionType :type "/Game/Blueprints/ENUM_InteractionTypes Enum" :default "NewEnumerator0") (CurrentFocusedActor :type "Actor Object Reference"))
  (if (`/Game/ThirdPerson/Blueprints/BP_Nyra.bIsInsideInteractRange` (`self.As BP Nyra`))
    (switch `/Game/Blueprints/ENUM_InteractionTypes` InteractionType
      (:`NewEnumerator0`
        (`/Game/ThirdPerson/Blueprints/BP_Nyra.OnEnterConversation` (`self.As BP Nyra`) CurrentFocusedActor))
      (:`NewEnumerator1`
        (bind _asbp_doorway (cast `/Game/Blueprints/BP_Doorway` CurrentFocusedActor))
        (`GameplayStatics.OpenLevelBySoftObjectPtr` (`/Game/Blueprints/BP_Doorway.WorldToLoad` _asbp_doorway))))))

(fn `SetMarkerVisibility`
  (params (InteractMarker :type "MeshComponent Object Reference") (Visibility :type Boolean))
  (`SceneComponent.SetHiddenInGame` InteractMarker (not Visibility) true)
  (`SceneComponent.K2_SetRelativeLocationAndRotation` InteractMarker (0.0 0.0 150.0) (`KismetMathLibrary.FindLookAtRotation` (`SceneComponent.K2_GetComponentLocation` InteractMarker) (`SceneComponent.K2_GetComponentLocation` (`/Game/ThirdPerson/Blueprints/BP_Nyra.DefaultCamera` (`self.As BP Nyra`)))) false false))