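; BP_Doorway is an interactable doorway that delegates its behavior to a BPCInteractable component linked to BP_Nyra.
; Its trigger box toggles the interact marker and Nyra's in-range flag, setting her focused actor on entry.
; E calls Interact on that focused actor, while Space exits conversations from this Blueprint because Nyra's input is disabled during them.
; PassNameToDialogueWidget sends the NameNotUsed value to Nyra's dialogue UI as the NPC name.
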(event `self.TriggerBox.OnComponentBeginOverlap`
  (params (OverlappedComponent :type "PrimitiveComponent Object Reference") (OtherActor :type "Actor Object Reference") (OtherComp :type "PrimitiveComponent Object Reference") (OtherBodyIndex :type Integer) (bFromSweep :type Boolean) (SweepResult :type "HitResult Structure (by ref)"))
  (bind _as_bp_nyra (`/Game/Blueprints/BPC_Interactable.As BP Nyra` (`self.BPC_Interactable`)))
  ; BP_Nyra HAS to keep score if she's inside the interact range
  (set `/Game/ThirdPerson/Blueprints/BP_Nyra.CurrentFocusedActor` (`ActorComponent.GetOwner` OverlappedComponent) _as_bp_nyra)
  (set `/Game/ThirdPerson/Blueprints/BP_Nyra.bIsInsideInteractRange` true _as_bp_nyra)
  (`/Game/Blueprints/BPC_Interactable.SetMarkerVisibility` (`self.BPC_Interactable`) (`self.WP_InteractMarker`) true))

(event `Key|SpaceBar`
  (params (Key :type "Key Structure"))
  ; Exiting from conversation always happens from here as input to Nyra is disabled
  (:`Pressed`
    (`/Game/ThirdPerson/Blueprints/BP_Nyra.OnExitConversation` (`/Game/Blueprints/BPC_Interactable.As BP Nyra` (`self.BPC_Interactable`)))))

(event `Key|E`
  (params (Key :type "Key Structure"))
  ; BP_Nyra HAS to keep score of currently focused actor, or it doesn't work
  (:`Pressed`
    (`/Game/Blueprints/BPC_Interactable.Interact` (`self.BPC_Interactable`) "NewEnumerator1" (`/Game/ThirdPerson/Blueprints/BP_Nyra.CurrentFocusedActor` (`/Game/Blueprints/BPC_Interactable.As BP Nyra` (`self.BPC_Interactable`))))))

(event `self.TriggerBox.OnComponentEndOverlap`
  (params (OverlappedComponent :type "PrimitiveComponent Object Reference") (OtherActor :type "Actor Object Reference") (OtherComp :type "PrimitiveComponent Object Reference") (OtherBodyIndex :type Integer))
  (`/Game/Blueprints/BPC_Interactable.SetMarkerVisibility` (`self.BPC_Interactable`) (`self.WP_InteractMarker`) false)
  (set `/Game/ThirdPerson/Blueprints/BP_Nyra.bIsInsideInteractRange` false (`/Game/Blueprints/BPC_Interactable.As BP Nyra` (`self.BPC_Interactable`))))

(fn `PassNameToDialogueWidget`
  (`/Game/NPCs/WBP_Dialogue.SetNPCName` (`/Game/ThirdPerson/Blueprints/BP_Nyra.DialogUI` (`/Game/Blueprints/BPC_Interactable.As BP Nyra` (`self.BPC_Interactable`))) (`self.Name (not used)`)))

(fn `UserConstructionScript`)