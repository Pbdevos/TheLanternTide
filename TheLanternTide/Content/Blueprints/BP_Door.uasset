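; BP_Door is an interactable door that moves the game from one streamed level to another.
; Range changes show or hide its marker through BPCInteractable.
; Interacting plays a WBP_Transition fade, waits briefly, then starts loading WorldToLoad and unloading CurrentWorld by soft reference, both non-blocking.
; A helper passes a name to Nyra's dialogue UI, while the conversation-exit call is unconnected and never runs.
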(event `Key|SpaceBar`
  (params (Key :type "Key Structure"))
  ; Exiting from conversation always happens from here as input to Nyra is disabled
)

(event `/Game/Blueprints/BPI_Interactable.ToggleMarker`
  (params (InRange :type Boolean))
  (`/Game/Blueprints/BPC_Interactable.SetMarkerVisibility` (`self.BPC_Interactable`) InRange (`self.InteractableMarkerLocation`)))

(event `/Game/Blueprints/BPI_Interactable.Interact`
  (params (PlayerRef :type "/Game/Blueprints/BP_Nyra Object Reference"))
  (bind _returnvalue (`|CreateWidget` "/Game/Blueprints/WBP_Transition.WBP_Transition_C" (`GameplayStatics.GetPlayerController` 0)))
  (bind _output_get (set `self.TransitionFade` _returnvalue))
  (`UserWidget.AddToViewport` _output_get 0)
  (`/Game/Blueprints/WBP_Transition.PlayFadingAnim` (`self.TransitionFade`) 0.5)
  (`KismetSystemLibrary.Delay` 0.5)
  (`GameplayStatics.LoadStreamLevelBySoftObjectPtr` (`self.WorldToLoad`) true)
  (`GameplayStatics.UnloadStreamLevelBySoftObjectPtr` (`self.CurrentWorld`)))

(fn `PassNameToDialogueWidget`
  (`/Game/Blueprints/WBP_Dialogue.SetNPCName` (`/Game/Blueprints/BP_Nyra.DialogUI` (`/Game/Blueprints/BPC_Interactable.As BP Nyra` (`self.BPC_Interactable`))) (`self.Name (not used)`)))

(fn `UserConstructionScript`)