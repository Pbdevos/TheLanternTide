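; BP_Conversation is a self-destroying actor that runs a conversation between Nyra and the NPC she is focused on.
; On BeginPlay it plays a transition fade while staggered delays switch the view to the NPC, move Nyra to that NPC's conversation position, disable her input and show the dialogue widget.
; Space Bar fades again, removes the dialogue, returns view and input to Nyra, then destroys the actor.
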(event `self.ReceiveBeginPlay`
  (`|ExecutionSequence`
    (:`then_0`
      (bind _nyraref (`/Game/Blueprints/BPC_Interactable.GetNyraRef` (`self.BPC_Interactable`)))
      (set `self.Nyra Ref` _nyraref)
      (bind _returnvalue (`|CreateWidget` "/Game/Blueprints/WBP_Transition.WBP_Transition_C" (`GameplayStatics.GetPlayerController` 0)))
      (bind _output_get (set `self.Transition Fade` _returnvalue))
      (`UserWidget.AddToViewport` _output_get 0)
      (`/Game/Blueprints/WBP_Transition.PlayFadingAnim` (`self.Transition Fade`) 1.0))
    (:`then_1`
      (`KismetSystemLibrary.Delay` 0.5)
      (`self.EnableInput` (`GameplayStatics.GetPlayerController` 0))
      (bind _asbp_npc (cast `/Game/Blueprints/BP_NPC` (`/Game/Blueprints/BP_Nyra.CurrentFocusedActor` (`self.Nyra Ref`))))
      (set `self.CurrentFocusedNPC` _asbp_npc)
      (`self.SwitchCamera` true (`self.Nyra Ref`) (`self.CurrentFocusedNPC`))
      (`self.PositionNyra` (`self.CurrentFocusedNPC`))
      (`self.Toggle Player Input` false))
    (:`then_2`
      (`KismetSystemLibrary.Delay` 1.0)
      (bind _returnvalue_2 (`|CreateWidget` "/Game/Blueprints/WBP_Dialogue.WBP_Dialogue_C" (`GameplayStatics.GetPlayerController` 0)))
      (bind _output_get_2 (set `self.Dialogue UI` _returnvalue_2))
      (`UserWidget.AddToViewport` _output_get_2 0))))

(event `Key|SpaceBar`
  (params (Key :type "Key Structure"))
  (bind _transition_fade (`self.Transition Fade`))
  (bind _dialogue_ui (`self.Dialogue UI`))
  (:`Pressed`
    (`UserWidget.AddToViewport` _transition_fade 0)
    (`/Game/Blueprints/WBP_Transition.PlayFadingAnim` _transition_fade 1.0)
    (`/Engine/EditorBlueprintResources/StandardMacros.IsValid` _dialogue_ui
      (:`Is Valid`
        (`Widget.RemoveFromParent` _dialogue_ui)
        (`KismetSystemLibrary.Delay` 0.5)
        (`self.SwitchCamera` false (`self.Nyra Ref`) (`self.CurrentFocusedNPC`))
        (`self.Toggle Player Input` true)
        (`self.DisableInput` (`GameplayStatics.GetPlayerController` 0))
        (`Widget.RemoveFromParent` (`self.Transition Fade`))
        (`self.K2_DestroyActor`)))))

(fn `PositionNyra`
  (params (NPC :type "/Game/Blueprints/BP_NPC Object Reference"))
  (`self.K2_SetActorTransform` (`self.Nyra Ref`) (`SceneComponent.K2_GetComponentToWorld` (`/Game/Blueprints/BP_NPC.NyraConversationPosition` NPC)) false false))

(fn `SwitchCamera`
  (params (InConversation :type Boolean) (Nyra :type "/Game/Blueprints/BP_Nyra Object Reference") (NPC :type "/Game/Blueprints/BP_NPC Object Reference"))
  (`PlayerController.SetViewTargetWithBlend` (`GameplayStatics.GetPlayerController` 0) (select `bool` InConversation :`false` Nyra :`true` NPC :!type "Actor Object Reference") 0.0 "VTBlend_Cubic" 0.0 false))

(fn `Toggle Player Input`
  (params (CanMove :type Boolean))
  (bind _returnvalue (`GameplayStatics.GetPlayerController` 0))
  (bind _nyra_ref (`self.Nyra Ref`))
  (if CanMove
    (`self.EnableInput` _nyra_ref _returnvalue)
    (else
      (`self.DisableInput` _nyra_ref _returnvalue))))

(fn `UserConstructionScript`)